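; BP_MovingGear is a moving hazard pawn that drives forward every tick and knocks away characters it hits.
; FloatingPawnMovement takes its max speed on BeginPlay, and a life span cleans the gear up automatically.
; On authority, GearCollision overlaps play a crash sound, launch BP_Character away and upward, then send CollidedMessage after a short delay.
; Set_CollisionVolume offsets the collision forward in proportion to speed, though nothing here calls it.
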(event OnComponentBeginOverlap(GearCollision)
  (params (OverlappedComponent :type Primitive%20Component%20Object%20Reference) (OtherActor :type Actor%20Object%20Reference) (OtherComp :type Primitive%20Component%20Object%20Reference) (OtherBodyIndex :type Integer) (bFromSweep :type Boolean) (SweepResult :type Hit%20Result%20Structure%20%28by%20ref%29))
  (bind _self self)
  ;[0.05098 0.05098 0.05098] Forwards the Collided event to the character that was hit by the Gear
  (Networking|SwitchHasAuthority
    (:Authority
      (bind _asbp_character (Utilities|Casting|CastToBP_Character OtherActor))
      (Audio|PlaySoundatLocation "/Game/_STUDENT_CONTENT/Project_Assets/Environment/SoundFX/SW_CarCrash.SW_CarCrash" (Transformation|GetActorLocation _asbp_character) "0, 0, 0" 1.0 1.0 0.0 "/Game/ParkourRace/Assets/Audio/Classes/SA_Short.SA_Short" 0 0 0)
      (Character|LaunchCharacter _asbp_character (* (Math|Vector|Normalize (+ (Math|Vector|Normalize (- (Transformation|GetActorLocation _asbp_character) (Transformation|GetActorLocation _self))) "0.000000,0.000000,1.500000")) (Variables|Default|GetLaunchStrength)) true true)
      (Utilities|FlowControl|Delay 0.1)
      (Class|BPINTGameplay|Collided(Message) _asbp_character _self))))

(event Custom|Set_CollisionVolume
  ;[0.15 0.15 0.15 0.5] Set Collision as Car Moves
  (Transformation|SetRelativeLocation (Variables|Default|GetGearCollision) (Math|Vector|MakeVector (Math|Float|MapRangeClamped (Math|Vector|VectorLength (Variables|/Script/Engine.MovementComponent|GetVelocity (Variables|Default|GetFloatingPawnMovement))) 0.0 (Variables|Default|GetMaxSpeed) 0.0 1e+02) 0.0 0.0) false false))

(event EventBeginPlay
  ;[0.15 0.15 0.15 0.5] Set Max Speed + Auto Clean Up
  (Variables|/Script/Engine.FloatingPawnMovement|SetMaxSpeed (Variables|Default|GetFloatingPawnMovement) (Variables|Default|GetMaxSpeed))
  (Actor|SetLifeSpan (Variables|Default|GetLifeSpan)))

(event Collision|EventActorBeginOverlap
  (params (OtherActor :type Actor%20Object%20Reference)))

(event EventTick
  (params (DeltaSeconds :type Float%20%28single-precision%29))
  ;[0.15 0.15 0.15 0.5] GearMovement
  (Pawn|Input|AddMovementInput (Transformation|GetActorForwardVector) 1.0 false))

(fn ConstructionScript)