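; Swinging pendulum hazard that knocks characters away on contact.
; Tick drives the pivot's roll with a sine of game time and plays an attenuated bell once at each swing extreme, using a resettable DoOnce.
; On the authority only, a box overlap with BP_Character plays a crash sound and launches it away with upward bias, then sends it CollidedMessage after a short delay.
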(event OnComponentBeginOverlap(Box)
  (params (OverlappedComponent :type Primitive%20Component%20Object%20Reference) (OtherActor :type Actor%20Object%20Reference) (OtherComp :type Primitive%20Component%20Object%20Reference) (OtherBodyIndex :type Integer) (bFromSweep :type Boolean) (SweepResult :type Hit%20Result%20Structure%20%28by%20ref%29))
  (bind _self self)
  ;[0.05098 0.05098 0.05098] Forwards the Collided event to the character that was hit by the pendulum
  (Networking|SwitchHasAuthority
    (:Authority
      (bind _asbp_character (Utilities|Casting|CastToBP_Character OtherActor))
      (Audio|PlaySoundatLocation "/Game/_STUDENT_CONTENT/Project_Assets/Environment/SoundFX/SW_CarCrash.SW_CarCrash" (Transformation|GetActorLocation _asbp_character) "0, 0, 0" 1.0 1.0 0.0 0 0 0 0)
      (Character|LaunchCharacter _asbp_character (* (Math|Vector|Normalize (+ (Math|Vector|Normalize (- (Transformation|GetActorLocation _asbp_character) (Transformation|GetActorLocation _self))) "0.000000,0.000000,1.500000")) (Variables|Default|GetLaunchStrength)) true true)
      (Utilities|FlowControl|Delay 0.1)
      (Class|BPINTGameplay|Collided(Message) _asbp_character _self))))

(event EventBeginPlay)

(event Collision|EventActorBeginOverlap
  (params (OtherActor :type Actor%20Object%20Reference)))

(event EventTick
  (params (DeltaSeconds :type Float%20%28single-precision%29))
  (bind _returnvalue (Utilities|Time|GetGameTimeinSeconds))
  (bind _returnvalue_2 (* _returnvalue 1.75))
  (bind _returnvalue_3 (Math|Trig|Sin(Radians) _returnvalue_2))
  ;[0.15 0.15 0.15 0.5] Pendulum Movement + Sound
  (Transformation|SetRelativeRotation (Variables|Default|GetSwingPivot) (Math|Rotator|MakeRotator (* _returnvalue_3 35.0) 0.0 0.0) true false)
  (if (> (Math|Float|Absolute(Float) _returnvalue_3) 0.99)
    (Utilities|FlowControl|DoOnce false :!label _label
      (:Completed
        (Audio|PlaySoundatLocation "/Game/_STUDENT_CONTENT/Project_Assets/Environment/SoundFX/SW_BellSound.SW_BellSound" (Transformation|GetActorLocation) "0, 0, 0" 1.0 1.0 0.0 "/Game/_STUDENT_CONTENT/Project_Assets/Environment/SoundFX/SA_Bell.SA_Bell" 0 0 0)))
    (else
      (goto _label Reset))))

(fn ConstructionScript)